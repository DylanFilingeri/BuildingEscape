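; Openable door Blueprint that swings open and closed in response to requests from its OpenDoor event source.
; It caches its starting rotation at BeginPlay, then the DoorSwing timeline adds an animated yaw to that rotation.
; An open request plays the timeline and a close request reverses it, while a timeline event track plays the door lock sound at the actor's location.
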(event `self.ReceiveBeginPlay`
  (set `self.InitialDoorRotation` (`self.K2_GetActorRotation`)))

(event `self.OpenDoor.OnOpenRequest`
  (bind (_direction _doorangle) (`Timeline|DoorSwing` :!label _label)
    (:`Update`
      (`self.K2_SetActorRotation` (`KismetMathLibrary.ComposeRotators` (`KismetMathLibrary.MakeRotator` 0.0 0.0 _doorangle) (`self.InitialDoorRotation`))))
    (:`SoundTiming`
      (`GameplayStatics.PlaySoundAtLocation` "/Game/Sounds/door-lock.door-lock" (`self.K2_GetActorLocation`)))))

(event `self.OpenDoor.OnCloseRequest`
  (goto _label :!via `Reverse`))

(fn `UserConstructionScript`)